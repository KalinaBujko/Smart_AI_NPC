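; BP_Sword is a sword pickup that the player collects by pressing E while nearby.
; Overlap events on the PickupRadius component toggle a PlayerInRange flag and print debug strings, without checking which actor overlaps.
; While the flag is set, Tick polls the E key directly on the player controller, then sets HasSword on BP_FirstPersonCharacter and destroys the pickup.
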(event `self.ReceiveTick`
  (params (DeltaSeconds :type "Float (single-precision)"))
  (if (`self.PlayerInRange`)
    (if (`PlayerController.IsInputKeyDown` (`GameplayStatics.GetPlayerController` 0) "E")
      (bind _asbp_first_person_character (cast `/Game/FirstPerson/Blueprints/BP_FirstPersonCharacter` (`GameplayStatics.GetPlayerCharacter` 0)))
      (set `/Game/FirstPerson/Blueprints/BP_FirstPersonCharacter.HasSword` true _asbp_first_person_character)
      (`self.K2_DestroyActor`))))

(event `self.PickupRadius_0.OnComponentBeginOverlap`
  (params (OverlappedComponent :type "PrimitiveComponent Object Reference") (OtherActor :type "Actor Object Reference") (OtherComp :type "PrimitiveComponent Object Reference") (OtherBodyIndex :type Integer) (bFromSweep :type Boolean) (SweepResult :type "HitResult Structure (by ref)"))
  (`KismetSystemLibrary.PrintString` "Player entered range")
  (set `self.PlayerInRange` true))

(event `self.PickupRadius_0.OnComponentEndOverlap`
  (params (OverlappedComponent :type "PrimitiveComponent Object Reference") (OtherActor :type "Actor Object Reference") (OtherComp :type "PrimitiveComponent Object Reference") (OtherBodyIndex :type Integer))
  (`KismetSystemLibrary.PrintString` "Player exit range")
  (set `self.PlayerInRange` false))

(fn `UserConstructionScript`)